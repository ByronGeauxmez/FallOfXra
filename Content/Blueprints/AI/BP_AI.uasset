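; BP_AI is an AI character that seeds its Blackboard with start location, roaming range and default behavior.
; Pawn sensing stores the first sighted player as the Blackboard Enemy, using a BBData helper for key access.
; A damage handler holds one-time ragdoll death and delayed destruction, but its binding never runs and it multiplies damage by zero.
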(event OnSeePawn(PawnSensing)
  (params (Pawn :type Pawn%20Object%20Reference))
  (bind (_returnvalue _returnvalue2) (CallFunction|BBData "Enemy"))
  (if (== Pawn (Game|GetPlayerCharacter 0))
    (Variables|Default|GetEnemyPawn
      (:then)
      (:else
        (bind _output_get (Variables|Default|SetEnemyPawn Pawn))
        (AI|Components|Blackboard|SetValueasObject _returnvalue _returnvalue2 _output_get)))))

(event Custom|OnTakeAnyDamage_Event_0
  (params (DamagedActor :type Actor%20Object%20Reference) (Damage :type Float%20%28single-precision%29) (DamageType :type Damage%20Type%20Object%20Reference) (InstigatedBy :type Controller%20Object%20Reference) (DamageCauser :type Actor%20Object%20Reference))
  (bind _mesh (Variables|Character|GetMesh))
  (bind _output_get (Variables|AI_Settings|SetHealth (- (Variables|AI_Settings|GetHealth) (* Damage 0.0))))
  (if (<= _output_get 0.0)
    (Utilities|FlowControl|DoOnce false
      (:Completed
        (Components|Activation|Deactivate (Variables|Default|GetAudio))
        (Collision|SetCollisionEnabled _mesh "PhysicsOnly")
        (Physics|SetSimulatePhysics _mesh true)
        (Physics|AddRadialImpulse _mesh "0, 0, 0" 0.0 0.0 "RIF_Constant" true)
        (Collision|SetCollisionEnabled (Variables|Collision|GetCapsuleComponent) "NoCollision")
        (Utilities|FlowControl|Delay 5.0)
        (Actor|DestroyActor)))))

(event Collision|EventActorBeginOverlap
  (params (OtherActor :type Actor%20Object%20Reference)))

(event EventTick
  (params (DeltaSeconds :type Float%20%28single-precision%29)))

(event EventBeginPlay
  (bind (_returnvalue _returnvalue2) (CallFunction|BBData "RoamingRange"))
  (bind (_returnvalue_2 _returnvalue2_2) (CallFunction|BBData "DefaultBehavior"))
  (bind (_returnvalue_3 _returnvalue2_3) (CallFunction|BBData "StartLocation"))
  (Variables|Default|SetStartLocation (Transformation|GetActorLocation))
  (AI|Components|Blackboard|SetValueasFloat _returnvalue _returnvalue2 (Variables|AI_Settings|GetMax_Wander_Distance))
  (AI|Components|Blackboard|SetValueasEnum _returnvalue_2 _returnvalue2_2 (Variables|AI_Settings|GetDefault_Behavior))
  (AI|Components|Blackboard|SetValueasVector _returnvalue_3 _returnvalue2_3 (Variables|Default|GetStartLocation)))

(fn ConstructionScript)

(fn BBData
  (params (KeyName :type Name))
  (return (AI|GetBlackboard (AI|GetAIController self)) (Utilities|Name|MakeLiteralName KeyName)))