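; Enemy AI character that wanders, chases the player once seen and damages them on box overlap.
; BeginPlay seeds the Blackboard with start location, roaming range and default behavior; pawn sensing sets the enemy key and raises speed.
; ReceiveDamage ragdolls and destroys it at zero health, but scales damage to zero.
; WIP AnyDamage plays a death montage and destroys it on any hit unless health is negative.
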(event OnSeePawn(PawnSensing)
  (params (Pawn :type Pawn%20Object%20Reference))
  (bind (_returnvalue _returnvalue2) (CallFunction|BBData "Enemy"))
  (bind _mesh (Variables|Character|GetMesh))
  ;[1 1 1] Seeing Player through pawn sensing
  (if (== Pawn (Game|GetPlayerCharacter 0))
    (Variables|Default|GetEnemyPawn
      (:then)
      (:else
        (bind _output_get (Variables|Default|SetEnemyPawn Pawn))
        (AI|Components|Blackboard|SetValueasObject _returnvalue _returnvalue2 _output_get)
        (Variables|/Script/Engine.CharacterMovementComponent|SetMaxWalkSpeed (Variables|Character|GetCharacterMovement) 6e+02)
        (Default|CallPlayerSpotted)
        (Animation|PlayAnimMontage "/Game/Characters/Mannequins/Animations/Manny/MM_Run_Fwd_Montage.MM_Run_Fwd_Montage" 1.0 "None")
        ;[1 1 1] Damage taken
        (if (<= (stale Custom|Event%20Receive%20Damage _output_get) 0.0)
          (Utilities|FlowControl|DoOnce false
            (:Completed
              (Default|CallDied)
              (Animation|StopAnimMontage "/Game/Characters/Mannequins/Animations/Manny/MM_Run_Fwd_Montage.MM_Run_Fwd_Montage")
              (Variables|/Script/Engine.CharacterMovementComponent|SetMaxWalkSpeed (Variables|Character|GetCharacterMovement) 0.0)
              (Components|Activation|Deactivate (Variables|Default|GetAudio))
              (Collision|SetCollisionEnabled _mesh "PhysicsOnly")
              (Physics|SetSimulatePhysics _mesh true)
              (Physics|AddRadialImpulse _mesh "0, 0, 0" 25.0 2e+03 "RIF_Constant" true)
              (Collision|SetCollisionEnabled (Variables|Collision|GetCapsuleComponent) "NoCollision")
              (Utilities|FlowControl|Delay 5.0)
              (Actor|DestroyActor))))))))

(event OnComponentBeginOverlap(Box)
  (params (OverlappedComponent :type Primitive%20Component%20Object%20Reference) (OtherActor :type Actor%20Object%20Reference) (OtherComp :type Primitive%20Component%20Object%20Reference) (OtherBodyIndex :type Integer) (bFromSweep :type Boolean) (SweepResult :type Hit%20Result%20Structure%20%28by%20ref%29))
  (bind _asbp_third_person_character (Utilities|Casting|CastToBP_ThirdPersonCharacter OtherActor))
  (Game|Damage|ApplyDamage _asbp_third_person_character 1e+01 0 self))

(event Custom|Event%20Receive%20Damage
  (params (Damage :type Float%20%28double-precision%29))
  (bind _mesh (Variables|Character|GetMesh))
  ;[1 1 1] Damage taken
  (bind _output_get (Variables|AISettings|SetHealth (- (Variables|AISettings|GetHealth) (* Damage 0.0))))
  (if (<= _output_get 0.0)
    (Utilities|FlowControl|DoOnce false
      (:Completed
        (Default|CallDied)
        (Animation|StopAnimMontage "/Game/Characters/Mannequins/Animations/Manny/MM_Run_Fwd_Montage.MM_Run_Fwd_Montage")
        (Variables|/Script/Engine.CharacterMovementComponent|SetMaxWalkSpeed (Variables|Character|GetCharacterMovement) 0.0)
        (Components|Activation|Deactivate (Variables|Default|GetAudio))
        (Collision|SetCollisionEnabled _mesh "PhysicsOnly")
        (Physics|SetSimulatePhysics _mesh true)
        (Physics|AddRadialImpulse _mesh "0, 0, 0" 25.0 2e+03 "RIF_Constant" true)
        (Collision|SetCollisionEnabled (Variables|Collision|GetCapsuleComponent) "NoCollision")
        (Utilities|FlowControl|Delay 5.0)
        (Actor|DestroyActor)))))

(event EventBeginPlay
  (bind (_returnvalue _returnvalue2) (CallFunction|BBData "StartLocation"))
  (bind (_returnvalue_2 _returnvalue2_2) (CallFunction|BBData "RoamingRange"))
  (bind (_returnvalue_3 _returnvalue2_3) (CallFunction|BBData "DefaultBehavior"))
  ;[1 1 1] Wandering Distance
  (bind _output_get (Variables|Default|SetStartLocation (Transformation|GetActorLocation)))
  (bind _output_get_2 (Variables|AI_Settings|SetMax_Wander_Distance (.Pitch (Math|Rotator|BreakRotator (Math|Conversions|RotationFromXVector _output_get)))))
  (AI|Components|Blackboard|SetValueasFloat _returnvalue_2 _returnvalue2_2 _output_get_2)
  (AI|Components|Blackboard|SetValueasEnum _returnvalue_3 _returnvalue2_3 (Variables|AI_Settings|GetDefault_Behavior))
  (AI|Components|Blackboard|SetValueasVector _returnvalue _returnvalue2 (Variables|Default|GetStartLocation))
  (Variables|/Script/Engine.CharacterMovementComponent|SetMaxWalkSpeed (Variables|Character|GetCharacterMovement) 2.5e+02))

(event Collision|EventActorBeginOverlap
  (params (OtherActor :type Actor%20Object%20Reference)))

(event EventTick
  (params (DeltaSeconds :type Float%20%28single-precision%29))
  ;[1 1 1] Wandering Distance
)

(event Game|Damage|EventAnyDamage
  (params (Damage :type Float%20%28single-precision%29) (DamageType :type Damage%20Type%20Object%20Reference) (InstigatedBy :type Controller%20Object%20Reference) (DamageCauser :type Actor%20Object%20Reference))
  ;[1 1 1] Combat System WIP - Set enemy health. takes damage. dies
  (if (< (Variables|AISettings|GetHealth) 0.0)
    (Variables|AISettings|SetHealth (- (Variables|AISettings|GetHealth) Damage))
    (else
      (Animation|StopAnimMontage "/Game/Characters/Mannequins/Animations/Manny/MM_Run_Fwd_Montage.MM_Run_Fwd_Montage")
      (Variables|/Script/Engine.CharacterMovementComponent|SetMaxWalkSpeed (Variables|Character|GetCharacterMovement) 0.0)
      (Utilities|FlowControl|Delay 0.5)
      (Animation|PlayAnimMontage "/Game/ThirdPerson/retargetedANIM/DummyDeath.DummyDeath" 1.25 "None")
      (Utilities|FlowControl|Delay 1.0)
      (Actor|DestroyActor))))

(fn ConstructionScript)

(fn BBData
  (params (KeyName :type Name))
  (return (AI|GetBlackboard (AI|GetAIController self)) (Utilities|Name|MakeLiteralName KeyName)))