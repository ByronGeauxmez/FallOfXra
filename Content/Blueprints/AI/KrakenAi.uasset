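; Kraken enemy character that chases the player and attacks with a two-hit sweep montage.
; Pawn sensing triggers an AI move to the player, with the attack on arrival, while a box overlap applies damage to the third-person character.
; ReceiveDamage holds a ragdoll death but multiplies damage by zero.
; The work-in-progress AnyDamage handler plays a death montage and destroys the actor unless health is already negative.
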(event OnSeePawn(PawnSensing)
  (params (Pawn :type Pawn%20Object%20Reference))
  (Variables|Default|SetIsSeePlayer true)
  (CallFunction|FollowPlayer))

(event OnComponentBeginOverlap(Box)
  (params (OverlappedComponent :type Primitive%20Component%20Object%20Reference) (OtherActor :type Actor%20Object%20Reference) (OtherComp :type Primitive%20Component%20Object%20Reference) (OtherBodyIndex :type Integer) (bFromSweep :type Boolean) (SweepResult :type Hit%20Result%20Structure%20%28by%20ref%29))
  (bind _asbp_third_person_character (Utilities|Casting|CastToBP_ThirdPersonCharacter OtherActor))
  (Game|Damage|ApplyDamage _asbp_third_person_character 1e+01 0 self))

(event Custom|Event%20Receive%20Damage
  (params (Damage :type Float%20%28double-precision%29))
  (bind _mesh (Variables|Character|GetMesh))
  ;[1 1 1] Damage Taken
  (bind _output_get (Variables|Default|SetHealth (- (Variables|Default|GetHealth) (* Damage 0.0))))
  (if (<= _output_get 0.0)
    (Utilities|FlowControl|DoOnce false
      (:Completed
        (Default|CallDied)
        (Animation|StopAnimMontage "/Game/Characters/Mannequins/Animations/Manny/MM_Run_Fwd_Montage.MM_Run_Fwd_Montage")
        (Variables|/Script/Engine.CharacterMovementComponent|SetMaxWalkSpeed (Variables|Character|GetCharacterMovement) 0.0)
        (Components|Activation|Deactivate (Variables|Default|GetAudio))
        (Collision|SetCollisionEnabled _mesh "PhysicsOnly")
        (Physics|SetSimulatePhysics _mesh true)
        (Physics|AddRadialImpulse _mesh "0, 0, 0" 25.0 2e+03 "RIF_Constant" true)
        (Collision|SetCollisionEnabled (Variables|Collision|GetCapsuleComponent) "NoCollision")
        (Utilities|FlowControl|Delay 5.0)
        (Actor|DestroyActor)))))

(event Custom|FollowPlayer
  (Variables|Default|SetcanAttack true)
  (if (Variables|Default|GetIsSeePlayer)
    (AI|AIMoveTo self "0, 0, 0" (Game|GetPlayerCharacter 0) 5.0 false
      (:OnSuccess
        (if (Variables|Default|GetcanAttack)
          (Variables|Default|SetcanAttack true)
          (bind _returnvalue (Animation|PlayAnimMontage "/Game/Kraken/Animations/KRAKEN_sweepAttack2HitCombo_Montage.KRAKEN_sweepAttack2HitCombo_Montage" 1.0 "None"))
          (Utilities|FlowControl|Delay _returnvalue)
          (Variables|Default|SetcanAttack true)
          (else
            (Variables|Default|SetcanAttack false)))))))

(event EventBeginPlay
  (if true
    (Components|Animation|PlayAnimation (Variables|Character|GetMesh) "/Game/Kraken/Animations/KRAKEN_idle.KRAKEN_idle" true)))

(event Collision|EventActorBeginOverlap
  (params (OtherActor :type Actor%20Object%20Reference)))

(event EventTick
  (params (DeltaSeconds :type Float%20%28single-precision%29)))

(event Game|Damage|EventAnyDamage
  (params (Damage :type Float%20%28single-precision%29) (DamageType :type Damage%20Type%20Object%20Reference) (InstigatedBy :type Controller%20Object%20Reference) (DamageCauser :type Actor%20Object%20Reference))
  ;[1 1 1] Combat System WIP
  (if (< (Variables|Default|GetHealth) 0.0)
    (Variables|Default|SetHealth (- (Variables|Default|GetHealth) Damage))
    (else
      (Animation|StopAnimMontage "/Game/Characters/Mannequins/Animations/Manny/MM_Run_Fwd_Montage.MM_Run_Fwd_Montage")
      (Variables|/Script/Engine.CharacterMovementComponent|SetMaxWalkSpeed (Variables|Character|GetCharacterMovement) 0.0)
      (Utilities|FlowControl|Delay 0.5)
      (Animation|PlayAnimMontage "/Game/ThirdPerson/retargetedANIM/DummyDeath.DummyDeath" 1.25 "None")
      (Utilities|FlowControl|Delay 0.25)
      (Actor|DestroyActor))))

(fn ConstructionScript)

(fn BBData
  (params (KeyName :type Name))
  (return 0 "None"))