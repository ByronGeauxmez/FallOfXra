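; Work-in-progress dummy combat enemy that reacts to sight and damage.
; PawnSensing sets a seeing flag, never cleared here, and calls FollowPlayer, which issues AIMoveTo with no target shown.
; AnyDamage subtracts damage only while Health is below zero; otherwise it plays the death montage between delays and destroys the actor.
; The health check appears inverted, so any hit at non-negative Health is fatal.
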(event OnSeePawn(PawnSensing)
  (params (Pawn :type Pawn%20Object%20Reference))
  ;[1 1 1] AI Detection
  (Variables|Default|SetisSeeingPlayer true)
  (CallFunction|FollowPlayer))

(event Custom|FollowPlayer
  ;[1 1 1] AI Detection
  (if (Variables|Default|GetisSeeingPlayer)
    (AI|AIMoveTo 0 "0, 0, 0" 0 5.0 false)))

(event EventBeginPlay)

(event Collision|EventActorBeginOverlap
  (params (OtherActor :type Actor%20Object%20Reference)))

(event EventTick
  (params (DeltaSeconds :type Float%20%28single-precision%29)))

(event Game|Damage|EventAnyDamage
  (params (Damage :type Float%20%28single-precision%29) (DamageType :type Damage%20Type%20Object%20Reference) (InstigatedBy :type Controller%20Object%20Reference) (DamageCauser :type Actor%20Object%20Reference))
  ;[1 1 1] Combat System WIP - Set enemy health. takes damage. dies
  (if (< (Variables|Default|GetHealth) 0.0)
    (Variables|Default|SetHealth (- (Variables|Default|GetHealth) Damage))
    (else
      (Utilities|FlowControl|Delay 0.5)
      (Animation|PlayAnimMontage "/Game/ThirdPerson/retargetedANIM/DummyDeath.DummyDeath" 1.25 "None")
      (Utilities|FlowControl|Delay 1.0)
      (Actor|DestroyActor))))

(fn ConstructionScript)