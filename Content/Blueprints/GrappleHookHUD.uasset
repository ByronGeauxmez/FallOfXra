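; HUD Blueprint for the grapple hook that draws a target icon following the mouse cursor.
; On BeginPlay it creates a GrappleTargetWidget, sets its icon to the target point texture and adds it to the viewport.
; Every Tick it moves the icon's canvas slot to the owning player's DPI-scaled mouse position, with no target detection or snapping in this Blueprint.
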(event EventTick
  (params (DeltaSeconds :type Float%20%28single-precision%29))
  (bind _playerowner (Variables|Default|GetPlayerOwner))
  (bind (_locationx _locationy) (Class|WidgetLayoutLibrary|GetMousePositionScaledbyDPI _playerowner))
  ;[1 1 1] Update Grapple Target Icon Based on Mouse Position
  (bind _output_get (Variables|Default|SetImage%20New%20Location (Math|Vector|MakeVector _locationx _locationy 0.0)))
  (Class|CanvasPanelSlot|SetPosition (Class|WidgetLayoutLibrary|SlotasCanvasSlot (Variables|/Game/Grapple_Hook_Items/GrappleTargetWidget.GrappleTargetWidget_C|GetGrappleIcon (Variables|Default|GetGrapple%20Widget))) (Math|Conversions|ToVector2D(Vector) _output_get)))

(event EventBeginPlay
  (bind _returnvalue (UserInterface|CreateWidget "/Game/Grapple_Hook_Items/GrappleTargetWidget.GrappleTargetWidget_C"))
  (bind _output_get (Variables|Default|SetGrapple%20Widget _returnvalue))
  (bind _output_get_2 (Variables|Default|SetTexture "/Engine/EditorResources/S_TargetPoint.S_TargetPoint"))
  (Appearance|SetBrushfromTexture (Variables|/Game/Grapple_Hook_Items/GrappleTargetWidget.GrappleTargetWidget_C|GetGrappleIcon _output_get) _output_get_2 false)
  (UserInterface|Viewport|AddtoViewport (Variables|Default|GetGrapple%20Widget) 0))

(fn ConstructionScript)