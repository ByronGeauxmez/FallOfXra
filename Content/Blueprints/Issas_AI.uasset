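; Issas_AI is an AI-controlled enemy character that roams, chases pawns it sees, and takes damage.
; From BeginPlay it loops AIMoveTo to random nearby reachable points, pausing randomly after each successful move.
; PawnSensing redirects movement to the seen pawn, with a retriggerable delay resuming roaming shortly after sightings stop.
; Damage lowers Health behind a DoOnce gate that reopens after the non-lethal montage, but stays closed at zero Health.
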(event OnSeePawn(PawnSensing)
  (params (Pawn :type Pawn%20Object%20Reference))
  (Utilities|FlowControl|Sequence
    (:then_0
      (AI|AIMoveTo self "0, 0, 0" Pawn 5.0 false))
    (:then_1
      (Utilities|FlowControl|RetriggerableDelay 3.0)
      (CallFunction|EnemyRoam))))

(event Custom|Enemy%20Roam
  (AI|AIMoveTo self (.RandomLocation (AI|Navigation|GetRandomReachablePointinRadius (Transformation|GetActorLocation) 5e+02 0 0)) 0 5.0 false
    (:OnSuccess
      (Utilities|FlowControl|Delay (Math|Random|RandomFloatinRange 1.0 3.0))
      (CallFunction|EnemyRoam))))

(event Game|Damage|EventAnyDamage
  (params (Damage :type Float%20%28single-precision%29) (DamageType :type Damage%20Type%20Object%20Reference) (InstigatedBy :type Controller%20Object%20Reference) (DamageCauser :type Actor%20Object%20Reference))
  (Utilities|FlowControl|DoOnce false :!label _label
    (:Completed
      (bind _output_get (Variables|Default|Sethealth (- (Variables|Default|Gethealth) Damage)))
      (if (<= _output_get 0.0)
        (Animation|PlayAnimMontage 0 1.0 "None")
        (else
          (bind _returnvalue (Animation|PlayAnimMontage 0 1.0 "None"))
          (Utilities|FlowControl|Delay _returnvalue)
          (goto _label Reset))))))

(event Collision|EventActorBeginOverlap
  (params (OtherActor :type Actor%20Object%20Reference)))

(event EventTick
  (params (DeltaSeconds :type Float%20%28single-precision%29)))

(event EventBeginPlay
  (CallFunction|EnemyRoam))

(fn ConstructionScript)