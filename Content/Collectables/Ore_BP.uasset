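; Collectable ore pickup that bobs in place and adds to the player character's ore count on overlap.
; A Timeline lerps it up to 30 units above its spawn location.
; Box overlap increments CurrentOre on the other actor's instigator character, then, only if that actor implements Ore_Interact_BP, plays a sound, sends the collected message and destroys the ore.
; SetOreAmount restores the count on load through the ore's own instigator.
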(event OnComponentBeginOverlap(Box)
  (params (OverlappedComponent :type Primitive%20Component%20Object%20Reference) (OtherActor :type Actor%20Object%20Reference) (OtherComp :type Primitive%20Component%20Object%20Reference) (OtherBodyIndex :type Integer) (bFromSweep :type Boolean) (SweepResult :type Hit%20Result%20Structure%20%28by%20ref%29))
  ;[1 1 1] Ore Pick Up
  (bind _asbp_third_person_character (Utilities|Casting|CastToBP_ThirdPersonCharacter (Game|GetInstigator OtherActor)))
  (Math|Integer|IncrementInt (Variables|/Game/ThirdPerson/BP_ThirdPersonCharacter.BP_ThirdPersonCharacter_C|GetCurrentOre _asbp_third_person_character)
    (:%20%20
      (if (Utilities|DoesObjectImplementInterface OtherActor "/Game/Collectables/Ore_Interact_BP.Ore_Interact_BP_C")
        (Audio|PlaySound2D "/Game/Collectables/CoinCollectionSound.CoinCollectionSound" 0.1 1.0 0.0 0 0)
        (Class|OreInteractBP|OnOreCollected(Message) OtherActor)
        (Actor|DestroyActor)))))

(event Custom|SetOreAmount
  (params (OreAmount :type Integer))
  ;[1 1 1] Set Ore Amount On Load
  (bind _asbp_third_person_character (Utilities|Casting|CastToBP_ThirdPersonCharacter (Game|GetInstigator)))
  (Variables|/Game/ThirdPerson/BP_ThirdPersonCharacter.BP_ThirdPersonCharacter_C|SetCurrentOre _asbp_third_person_character OreAmount))

(event EventBeginPlay
  ;[1 1 1] Floating Logic
  (bind _output_get (Variables|Default|SetOriginLocation (Transformation|GetActorLocation)))
  (bind _alpha (Timeline|Timeline_0 Play)
    (:Update
      (Transformation|SetActorLocation (Math|Vector|Lerp(Vector) (Variables|Default|GetOriginLocation) (+ _output_get "0,0.000000,30.000000") _alpha) false false))))

(fn ConstructionScript)