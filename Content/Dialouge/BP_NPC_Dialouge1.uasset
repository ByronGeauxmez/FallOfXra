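; BP_NPC_Dialouge1 is an NPC dialogue Blueprint that steps through an array of lines each time its Talk event fires.
; Talk increments TalkIndex, creates a WB_Dialouge1 widget for the viewport if UI is invalid, and writes the current line to its TalkText.
; Once the index passes the last line, the widget is removed from its parent, and nothing here resets the index.
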(event Collision|EventActorBeginOverlap
  (params (OtherActor :type Actor%20Object%20Reference)))

(event EventTalk
  (Math|Integer|IncrementInt (Variables|Default|GettalkIndex)
    (:%20%20
      (if (< (Variables|Default|GettalkIndex) (Utilities|Array|Length (Variables|Default|Getdialouge)))
        (Variables|Default|GetUI
          (:then
            _)
          (:else
            (UserInterface|CreateWidget "/Game/Dialouge/WB_Dialouge1.WB_Dialouge1_C" (Game|GetPlayerController 0))
            (bind _output_get (Variables|Default|SetUI 0))
            (UserInterface|Viewport|AddtoViewport _output_get 0)))
        (Rendering|Components|TextRender|SetText (Variables|/Game/Dialouge/WB_Dialouge.WB_Dialouge_C|GetTalkText (Variables|Default|GetUI)) (Utilities|Text|ToText(String) (Utilities|Array|Get(acopy) (Variables|Default|Getdialouge) (Variables|Default|GettalkIndex))))
        (else
          (Widget|RemovefromParent (Variables|Default|GetUI)))))))

(fn ConstructionScript)