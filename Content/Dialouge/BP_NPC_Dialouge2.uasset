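; BP_NPC_Dialouge2 is an NPC dialogue Blueprint that shows the Dialouge2 lines one at a time in an on-screen widget.
; Each Talk event advances TalkIndex, lazily creates the UI widget if needed and sets its TalkText to the current line.
; Past the last line it removes the widget, but TalkIndex is never reset and the node clearing UI never runs.
; The overlap event and construction script are empty.
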(event Collision|EventActorBeginOverlap
  (params (OtherActor :type Actor%20Object%20Reference)))

(event EventTalk
  (Math|Integer|IncrementInt (Variables|Default|GettalkIndex)
    (:%20%20
      (if (< (Variables|Default|GettalkIndex) (Utilities|Array|Length (Variables|Default|Getdialouge2)))
        (Variables|Default|GetUI
          (:then
            _)
          (:else
            (bind _returnvalue (UserInterface|CreateWidget "/Game/Dialouge/WB_Dialouge2.WB_Dialouge2_C" (Game|GetPlayerController 0)))
            (bind _output_get (Variables|Default|SetUI _returnvalue))
            (UserInterface|Viewport|AddtoViewport _output_get 0)))
        (Rendering|Components|TextRender|SetText (Variables|/Game/Dialouge/WB_Dialouge2.WB_Dialouge2_C|GetTalkText (Variables|Default|GetUI)) (Utilities|Text|ToText(String) (Utilities|Array|Get(acopy) (Variables|Default|Getdialouge2) (Variables|Default|GettalkIndex))))
        (else
          (Widget|RemovefromParent (Variables|Default|GetUI)))))))

(fn ConstructionScript)